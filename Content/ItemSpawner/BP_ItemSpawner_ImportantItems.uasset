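; BP_ItemSpawner_ImportantItems is a spawner actor that places one random item from its ItemsToSpawnImp class list.
; On BeginPlay it calls AttemptToSpawn, which only prints a message if CurrentItem is still valid and otherwise calls SpawnItem.
; SpawnItem spawns the chosen class at the spawner's location and rotation with unit scale, owned by the spawner, and stores it as CurrentItem.
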(event `self.ReceiveBeginPlay`
  (`self.AttemptToSpawn`))

(fn `AttemptToSpawn`
  (`/Engine/EditorBlueprintResources/StandardMacros.IsValid` (`self.CurrentItem`)
    (:`Is Valid`
      (`KismetSystemLibrary.PrintString` "Item already Spawned"))
    (:`Is Not Valid`
      (`self.SpawnItem`))))

(fn `SpawnItem`
  (bind _returnvalue (`|SpawnActorFromClass` (`|GetArrayItem` (`self.ItemsToSpawnImp`) (`KismetMathLibrary.RandomIntegerInRange` 0 (- (`KismetArrayLibrary.Array_Length` (`self.ItemsToSpawnImp`)) 1))) (`KismetMathLibrary.MakeTransform` (`self.K2_GetActorLocation`) (`self.K2_GetActorRotation`)) "AdjustIfPossibleButAlwaysSpawn" "OverrideRootScale" self null))
  (set `self.CurrentItem` _returnvalue))

(fn `UserConstructionScript`)