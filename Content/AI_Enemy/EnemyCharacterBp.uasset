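; Enemy AI character that chases the player, attacks, and ragdolls on death.
; PawnSensing starts a chase on seeing the third-person character; each successful AI MoveTo calls ApplyDamage, with no damaged actor wired, then re-chases after a short delay.
; Incoming damage feeds the health system component, whose death dispatcher enables mesh physics.
; It also toggles a lock-on visual and exposes a distance-to-player check.
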(event `/Game/AI_Enemy/GameBPI.TargetLockOn`
  (bind _targetvisual (`self.TargetVisual`))
  ;[1 1 1] Target Lock On Event
  (`/Engine/EditorBlueprintResources/StandardMacros.FlipFlop`
    (:`A`
      (`SceneComponent.SetHiddenInGame` _targetvisual false false))
    (:`B`
      (`SceneComponent.SetHiddenInGame` _targetvisual true false))))

(event `self.ReceiveAnyDamage`
  (params (Damage :type "Float (single-precision)") (DamageType :type "DamageType Object Reference") (InstigatedBy :type "Controller Object Reference") (DamageCauser :type "Actor Object Reference"))
  (`/Game/ThirdPersonBP/EnemyHealthSytem.TakeDamage` (`self.EnemyHealthSytem`) Damage))

(event `self.EnemyHealthSytem.DeathDispatcher`
  (`PrimitiveComponent.SetSimulatePhysics` (`self.Mesh`) true))

(event `Chase`
  (params (`Player To Chase` :type "Pawn Object Reference"))
  ;[1 1 1] AI chase function
  (`|AIMoveTo` self (0.0 0.0 0.0) `Player To Chase`
    (:`OnSuccess`
      (`GameplayStatics.ApplyDamage` null (`self.Damge`))
      (`KismetSystemLibrary.Delay` 1.0)
      (`self.Chase` `Player To Chase`))))

(event `self.PawnSensing.OnSeePawn`
  (params (Pawn :type "Pawn Object Reference"))
  (bind _asthird_person_character (cast `/Game/ThirdPersonBP/Blueprints/ThirdPersonCharacter` Pawn))
  (`self.Chase` _asthird_person_character))

(fn `DistanceFromPlayerCheck`
  (returns (DistanceFromPlayer :type "Float (double-precision)"))
  (return (`self.GetDistanceTo` (`GameplayStatics.GetPlayerCharacter` 0))))

(fn `UserConstructionScript`)